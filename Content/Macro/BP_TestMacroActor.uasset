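; Test actor that exercises Blueprint-exposed properties and functions, apparently from a C++ parent, with results shown through Print String.
; It implements BlueprintImplementableEventFunction to scale a float and BlueprintNativeEventFunction to append a Blueprint tag to an actor's display name.
; BeginPlay prints the latter's result for itself.
; Pressing Z passes the getter/setter property back through itself and prints it, while other property test nodes sit unconnected.
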(event EventBeginPlay
  (bind _returnvalue (CallFunction|BlueprintNativeEventFunction self))
  (Development|PrintString _returnvalue))

(event Collision|EventActorBeginOverlap
  (params (OtherActor :type Actor%20Object%20Reference)))

(event EventTick
  (params (DeltaSeconds :type Float%20%28single-precision%29)))

(event Input|KeyboardEvents|Z
  (params (Key :type Key%20Structure :default "None"))
  (:Pressed
    (bind _output_get (Variables|Default|SetBlueprintGetterAndSetterParam (Variables|Default|GetBlueprintGetterAndSetterParam)))
    (Development|PrintString (Utilities|String|ToString(Float) _output_get))))

(fn ConstructionScript)

(fn BlueprintImplementableEventFunction
  (params (InFloat :type Float%20%28single-precision%29))
  (return (* InFloat 1e+01)))

(fn BlueprintNativeEventFunction
  (params (InActor :type Actor%20Object%20Reference))
  (return (Utilities|String|Append (Utilities|GetDisplayName InActor) "-" "Blueprint")))