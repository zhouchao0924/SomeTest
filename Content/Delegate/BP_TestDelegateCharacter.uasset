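; BP_TestDelegateCharacter is a test character for trying out C++ delegate types from Blueprint.
; Debug keys trigger native functions for binding, executing, multicast, event and dynamic delegate tests.
; On BeginPlay it runs the dynamic multicast test and binds a Blueprint event to a dynamic multicast delegate.
; Pressing Q broadcasts that delegate with a fixed code, which the bound event prints to screen.
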(event Custom|DynamicMulticastTest
  (params (nCode :type Integer))
  (Development|PrintString (Utilities|String|Append "DynamicMulticast:" (Utilities|String|ToString(Integer) nCode))))

(event EventBeginPlay
  (Class|TestDelegateCharacter|OnDelegateDynamicMulticastTest)
  (EventDispatchers|BindEventtoCharacterDelegateDynamicMulticast2 (delegate Custom|DynamicMulticastTest)))

(event Input|KeyboardEvents|Z
  (params (Key :type Key%20Structure :default "None"))
  (:Pressed
    (Class|TestDelegateCharacter|OnBind)))

(event Input|KeyboardEvents|X
  (params (Key :type Key%20Structure :default "None"))
  (:Pressed
    (Class|TestDelegateCharacter|OnExecute)))

(event Input|KeyboardEvents|C
  (params (Key :type Key%20Structure :default "None"))
  (:Pressed
    (Class|TestDelegateCharacter|OnDelegateMulticastTest)))

(event Input|KeyboardEvents|V
  (params (Key :type Key%20Structure :default "None"))
  (:Pressed
    (Class|TestDelegateCharacter|OnEventTest)))

(event Input|KeyboardEvents|B
  (params (Key :type Key%20Structure :default "None"))
  (:Pressed
    (Class|TestDelegateCharacter|OnDelegateDynamicTest)))

(event Input|KeyboardEvents|Q
  (params (Key :type Key%20Structure :default "None"))
  (:Pressed
    (Class|TestDelegateCharacter|BrocastCharacterDelegateDynamicMulticast 100)))

(fn ConstructionScript)