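; Test game mode Blueprint that calls TestFunc3 with default-looking arguments two seconds after BeginPlay.
; A separate EEERRR function prints its four inputs and returns fixed int, string, transform and bool outputs.
; Nothing in this Blueprint calls EEERRR, and TestFunc3 is defined outside it.
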(event EventBeginPlay
  (Utilities|FlowControl|Delay 2.0)
  (Class|SomeTestGameModeBase|TestFunc3 0 "" false))

(event EventTick
  (params (DeltaSeconds :type Float%20%28single-precision%29)))

(fn ConstructionScript)

(fn EEERRR
  (params (NewParam :type Rotator) (NewParam1 :type Integer) (NewParam2 :type String) (NewParam3 :type Object%20Object%20Reference))
  (Development|PrintString (Utilities|String|ToString(Rotator) NewParam))
  (Development|PrintString (Utilities|String|ToString(Integer) NewParam1))
  (Development|PrintString NewParam2)
  (Development|PrintString (Utilities|GetDisplayName NewParam3))
  (return 0 "qq" (Math|Transform|MakeTransform "1111.000000, 0, 0" "0, 0,12.000000" "1.000000,1,1") true))